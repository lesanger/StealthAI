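; Enemy AI controller that runs BT_EnemyBehavior on BeginPlay and feeds it sight perception through the Blackboard.
; Perception updates go to HandleSense, which matches the sense class by display name and handles only sight.
; Any sight update sets IsInvestigating to its success, but only the player character becomes InvestigatedCharacter.
; Losing sight stores the stimulus location in TargetLocationVector, clears InvestigatedCharacter and prints a debug string.
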(event `self.ReceiveBeginPlay`
  (`self.RunBehaviorTree` "/Game/EnemyAI/BT_EnemyBehavior.BT_EnemyBehavior"))

(event `self.AIPerception.OnTargetPerceptionUpdated`
  (params (Actor :type "Actor Object Reference") (Stimulus :type "AIStimulus Structure"))
  (bind _returnvalue (`AIPerceptionSystem.GetSenseClassForStimulus` Stimulus))
  (`self.HandleSense` _returnvalue Actor Stimulus))

(fn `HandleSense`
  (params (InClass :type "Object Object Reference") (InActor :type "Actor Object Reference") (InAIStimulus :type "AIStimulus Structure (by ref)"))
  (bind (_inaistimulus_age _inaistimulus_expirationage _inaistimulus_strength _inaistimulus_stimuluslocation) (break `AIStimulus` (`local.InAIStimulus`)))
  (bind (_inaistimulus_age_2 _inaistimulus_expirationage_2 _inaistimulus_strength_2 _inaistimulus_stimuluslocation_2 _inaistimulus_receiverlocation _inaistimulus_tag _inaistimulus_bsuccessfullysensed) (break `AIStimulus` (`local.InAIStimulus`)))
  (switch `string` (`KismetSystemLibrary.GetClassDisplayName` InClass)
    (:`AiSense_Sight`
      (`BlackboardComponent.SetValueAsBool` (`self.Blackboard`) "IsInvestigating" _inaistimulus_bsuccessfullysensed)
      (if _inaistimulus_bsuccessfullysensed
        (if (== (`local.InActor`) (`GameplayStatics.GetPlayerCharacter` 0))
          (`BlackboardComponent.SetValueAsObject` (`self.Blackboard`) "InvestigatedCharacter" (`local.InActor`)))
        (else
          (`BlackboardComponent.SetValueAsVector` (`self.Blackboard`) "TargetLocationVector" _inaistimulus_stimuluslocation)
          (`BlackboardComponent.SetValueAsObject` (`self.Blackboard`) "InvestigatedCharacter" null)
          (`KismetSystemLibrary.PrintString` "Hello"))))))

(fn `UserConstructionScript`)