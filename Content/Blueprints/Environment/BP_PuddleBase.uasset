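; Base puddle actor that plays a splash footstep sound and reports a noise event while the player overlaps it.
; Each Tick, if no sound instance is active, it spawns the puddle cue at the player's location with the player as noise instigator.
; A half-second delay then stops and clears the sound, pacing repeats.
; The velocity check (>= 0) always passes, so standing still also triggers it.
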(event `self.ReceiveTick`
  (params (DeltaSeconds :type "Float (single-precision)"))
  (bind _returnvalue (`GameplayStatics.GetPlayerCharacter` 0))
  (bind _returnvalue_2 (`self.K2_GetActorLocation` _returnvalue))
  (`self.SoundInstance`
    (:`then`)
    (:`else`
      (if (`self.IsOverlappingActor` _returnvalue)
        (if (>= (`KismetMathLibrary.VSize` (`self.GetVelocity` _returnvalue)) 0.0)
          (bind _returnvalue_3 (`GameplayStatics.SpawnSoundAtLocation` "/Game/Sound/SCue_FootStep_Puddle.SCue_FootStep_Puddle" _returnvalue_2 (struct) 1.0 1.0 0.0 null null))
          (set `self.SoundInstance` _returnvalue_3)
          (`AISense_Hearing.ReportNoiseEvent` _returnvalue_2 1.0 (`GameplayStatics.GetPlayerCharacter` 0))
          (`KismetSystemLibrary.Delay` 0.5)
          (`AudioComponent.Stop` (`self.SoundInstance`))
          (set `self.SoundInstance` null))))))

(fn `UserConstructionScript`)